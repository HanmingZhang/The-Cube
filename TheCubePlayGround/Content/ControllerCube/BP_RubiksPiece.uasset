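; BP_RubiksPiece is an actor for a single Rubik's cube piece, built from a static mesh and six text render components.
; The construction script gathers the six text renders into a Texts array.
; On BeginPlay it creates a dynamic material instance from Base on one element of the mesh and stores it in Mat.
; It has no other active logic of its own, as Tick and overlap are empty.
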(event `self.ReceiveBeginPlay`
  (bind _returnvalue (`PrimitiveComponent.CreateDynamicMaterialInstance` (`self.StaticMesh`) 6 "/Game/ControllerCube/Meshes/RubikPiece/Materials/base.base"))
  (set `self.Mat` _returnvalue))

(event `self.ReceiveTick`
  (params (DeltaSeconds :type "Float (single-precision)")))

(fn `UserConstructionScript`
  (set `self.Texts` (`|MakeArray` (`self.TextRender`) (`self.TextRender1`) (`self.TextRender2`) (`self.TextRender3`) (`self.TextRender4`) (`self.TextRender5`))))